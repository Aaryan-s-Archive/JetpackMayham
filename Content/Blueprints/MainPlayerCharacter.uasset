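; Player character that carries a rocket launcher, spawned on BeginPlay and attached to the mesh's weapon socket.
; Fire input, gated by a one-second cooldown, traces from the camera and aims the launcher from its muzzle at the hit point, else along control rotation.
; Aim events snap the camera boom length.
; When controller fuel is low, Tick runs forward then downward debug-drawn clamber sphere traces, without acting on the result; ActivateThrusters is empty.
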(event `self.ReceiveBeginPlay`
  (bind _returnvalue (`|SpawnActorFromClass` "/Game/Weapons/RocketLauncherBaseBP.RocketLauncherBaseBP_C" (`SceneComponent.K2_GetComponentToWorld` (`self.Mesh`)) "AlwaysSpawn" "OverrideRootScale"))
  (bind _output_get (set `self.SciFiRocketLauncher` _returnvalue))
  (`self.K2_AttachRootComponentTo` _output_get (`self.Mesh`) "WeaponSocket" "SnapToTarget" true)
  (bind _asmain_player_controller (cast `/Game/Blueprints/MainPlayerController` (`GameplayStatics.GetPlayerController` 0)))
  (set `self.ControllerCast` _asmain_player_controller))

(event `InputAction|FIRE`
  (params (Key :type "Key Structure" :default "AnyKey"))
  (bind _scifirocketlauncher (`self.SciFiRocketLauncher`))
  (bind _camera (`self.Camera`))
  (bind _returnvalue (`SceneComponent.K2_GetComponentLocation` _camera))
  (:`Pressed`
    (if (`self.Can Fire`)
      (set `self.Can Fire` false)
      (bind (_outhit _returnvalue_2) (`KismetSystemLibrary.LineTraceSingle` :`Start` _returnvalue :`End` (+ _returnvalue (* (`SceneComponent.GetForwardVector` _camera) 9999999.0)) :`TraceChannel` "TraceTypeQuery1" :`DrawDebugType` "ForDuration"))
      (if _returnvalue_2
        (`/Game/Weapons/RocketLauncherBaseBP.FireEvent` _scifirocketlauncher (`KismetMathLibrary.FindLookAtRotation` (`SceneComponent.GetSocketLocation` (`/Game/Weapons/RocketLauncherBaseBP.Weapon` (`self.SciFiRocketLauncher`)) "Muzzle") (`.ImpactPoint` (`GameplayStatics.BreakHitResult` _outhit))))
        (else
          (`/Game/Weapons/RocketLauncherBaseBP.FireEvent` _scifirocketlauncher (`self.GetControlRotation`))))
      (`KismetSystemLibrary.Delay` 1.0)
      (set `self.Can Fire` true))))

(event `ActivateThrusters`)

(event `Aim`
  (set `SpringArmComponent.TargetArmLength` 100.0 (`self.CameraBoom`)))

(event `NoAim`
  (set `SpringArmComponent.TargetArmLength` 200.0 (`self.CameraBoom`)))

(event `self.ReceiveTick`
  (params (DeltaSeconds :type "Float (single-precision)"))
  (bind _clambercube (`self.ClamberCube`))
  (bind _locationpoint (`self.LocationPoint`))
  (bind _returnvalue (`SceneComponent.K2_GetComponentLocation` _clambercube))
  (bind _returnvalue_2 (`SceneComponent.K2_GetComponentLocation` _locationpoint))
  (if (< (`/Game/Blueprints/MainPlayerController.Fuel` (`self.ControllerCast`)) 20)
    (bind (_outhit _returnvalue_3) (`KismetSystemLibrary.SphereTraceSingle_NEW` :`Start` _returnvalue :`End` (+ _returnvalue (* (`SceneComponent.GetForwardVector` _clambercube) 200.0)) :`Radius` 10.0 :`TraceChannel` "TraceTypeQuery1" :`DrawDebugType` "ForDuration"))
    (if _returnvalue_3
      (`KismetSystemLibrary.SphereTraceSingle_NEW` :`Start` _returnvalue_2 :`End` (+ _returnvalue_2 (* (* (`SceneComponent.GetUpVector` _locationpoint) -1.0) 200.0)) :`Radius` 10.0 :`TraceChannel` "TraceTypeQuery1" :`DrawDebugType` "ForDuration"))))

(fn `UserConstructionScript`)