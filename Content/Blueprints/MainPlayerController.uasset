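; Player controller that turns input into movement, camera look, jetpack thrust and aiming for the player character.
; Movement follows control yaw, and gamepad look is scaled by turn rate and delta time, unlike mouse look.
; Holding Jump runs a short Delay loop that drains fuel, adds upward force and activates thrusters until release or empty.
; Tick interpolates fuel back toward maximum while not falling, and Aim input calls the character's aim functions.
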(event `InputAxis|MoveForward`
  (params (AxisValue :type "Float (single-precision)"))
  ;[1 1 1] Movement
  (`Pawn.AddMovementInput` (`GameplayStatics.GetPlayerCharacter` 0) (`KismetMathLibrary.GetForwardVector` (`KismetMathLibrary.MakeRotator` 0.0 0.0 (.yaw (`self.GetControlRotation`)))) AxisValue false))

(event `InputAxis|MoveRight`
  (params (AxisValue :type "Float (single-precision)"))
  ;[1 1 1] Movement
  (`Pawn.AddMovementInput` (`GameplayStatics.GetPlayerCharacter` 0) (`KismetMathLibrary.GetRightVector` (`KismetMathLibrary.MakeRotator` 0.0 0.0 (.yaw (`self.GetControlRotation`)))) AxisValue false))

(event `InputAxis|MousePitch`
  (params (AxisValue :type "Float (single-precision)"))
  ;[1 1 1] MouseCamera
  (`self.AddPitchInput` AxisValue))

(event `InputAxis|MouseYaw`
  (params (AxisValue :type "Float (single-precision)"))
  ;[1 1 1] MouseCamera
  (`self.AddYawInput` AxisValue))

(event `InputAxis|GamepadYaw`
  (params (AxisValue :type "Float (single-precision)"))
  ;[1 1 1] Gamepad Camera Controls
  (`self.AddYawInput` (* AxisValue (`self.BaseTurnRate`) (`GameplayStatics.GetWorldDeltaSeconds`))))

(event `InputAxis|GamepadPitch`
  (params (AxisValue :type "Float (single-precision)"))
  ;[1 1 1] Gamepad Camera Controls
  (`self.AddPitchInput` (* AxisValue (`self.BaseTurnRate`) (`GameplayStatics.GetWorldDeltaSeconds`))))

(event `InputAction|Jump`
  (params (Key :type "Key Structure" :default "AnyKey"))
  (:`Pressed`
    (set `self.JumpButtonPressed` true)
    (bind _output_get (set `self.Fuel` (- (`self.Fuel`) (`self.LossAmount`)) :!label _label))
    (if (> _output_get 0)
      (`CharacterMovementComponent.AddForce` (`Character.CharacterMovement` (`GameplayStatics.GetPlayerCharacter` 0)) (`KismetMathLibrary.MakeVector` 0.0 0.0 (`self.JetpackZForce`)))
      (`/Game/Blueprints/MainPlayerCharacter.ActivateThrusters` (cast `/Game/Blueprints/MainPlayerCharacter` (`GameplayStatics.GetPlayerCharacter` 0) :!pure true))
      (`KismetSystemLibrary.Delay` 0.01)
      (if (`self.JumpButtonPressed`)
        (goto _label))))
  (:`Released`
    (set `self.JumpButtonPressed` false)))

(event `self.ReceiveTick`
  (params (DeltaSeconds :type "Float (single-precision)"))
  (`|ExecutionSequence`
    (:`then_0`
      (if (not (`NavMovementComponent.IsFalling` (`Pawn.GetMovementComponent` (`GameplayStatics.GetPlayerCharacter` 0))))
        (set `self.Fuel` (`KismetMathLibrary.FTrunc` (`KismetMathLibrary.FInterpTo` (`KismetMathLibrary.Conv_IntToDouble` (`self.Fuel`)) (`KismetMathLibrary.Conv_IntToDouble` (`self.FuelMax`)) (`GameplayStatics.GetWorldDeltaSeconds`) 5.0)))))))

(event `InputAction|Aim`
  (params (Key :type "Key Structure" :default "AnyKey"))
  (bind _asmain_player_character (cast `/Game/Blueprints/MainPlayerCharacter` (`GameplayStatics.GetPlayerCharacter` 0) :!pure true))
  (:`Pressed`
    (`/Game/Blueprints/MainPlayerCharacter.Aim` _asmain_player_character))
  (:`Released`
    (`/Game/Blueprints/MainPlayerCharacter.NoAim` _asmain_player_character)))

(fn `UserConstructionScript`)